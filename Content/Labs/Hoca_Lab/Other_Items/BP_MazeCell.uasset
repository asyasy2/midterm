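; BP_MazeCell is a configurable maze tile with optional walls, ceiling, point light and trap.
; The construction script scales the floor, adds meshes from the grid size and flags, and, only when lit, sets the light and trap child actor class.
; On BeginPlay it may randomly spawn a Medkit or Gold, and binds to the player's MazeGate event, recoloring its light to the player's color when IsInside is false.
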(event Custom|MazeGateEvent
  (params (IsInside? :type Boolean))
  (bind _pointlight (Variables|Default|GetPointLight))
  (if (not IsInside?)
    (Utilities|IsValid _pointlight
      (:Is%20Valid
        (Rendering|Components|Light|SetLightColor _pointlight (Variables|/Game/Labs/Hoca_Lab/BP_ThirdPersonCharacter.BP_ThirdPersonCharacter_C|GetLight%20Color (Variables|Default|GetAs%20BP%20Third%20Person%20Character)) true)))))

(event EventBeginPlay
  (bind _collectible_position (Variables|Default|GetCollectible%20position))
  (bind _returnvalue (Transformation|GetWorldLocation _collectible_position))
  (bind _asbp_third_person_character (Utilities|Casting|CastToBP_ThirdPersonCharacter (Game|GetPlayerCharacter 0)))
  (Variables|Default|SetAs%20BP%20Third%20Person%20Character _asbp_third_person_character)
  (EventDispatchers|BindEventtoMazeGate _asbp_third_person_character (delegate Custom|MazeGateEvent))
  (if (> (Math|Random|RandomIntegerinRange 0 10) 8)
    (Game|SpawnActorfromClass "/Game/Labs/Hoca_Lab/Other_Items/Medkit.Medkit_C" (Math|Transform|MakeTransform _returnvalue "0, 0, 0" "1.000000,1.000000,1.000000") "Undefined" "MultiplyWithRoot" 0 0)
    (elif (> (Math|Random|RandomIntegerinRange 0 10) 7)
      (Game|SpawnActorfromClass "/Game/Labs/Hoca_Lab/Other_Items/Gold.Gold_C" (Math|Transform|MakeTransform _returnvalue "0, 0, 0" "1.000000,1.000000,1.000000") "Undefined" "MultiplyWithRoot" 0 0))))

(event Collision|EventActorBeginOverlap
  (params (OtherActor :type Actor%20Object%20Reference)))

(event EventTick
  (params (DeltaSeconds :type Float%20%28single-precision%29)))

(fn ConstructionScript
  (bind _gridsize (Variables|Default|Getgridsize))
  (LocalVariables|Setwalllenght _gridsize)
  (LocalVariables|Setwallthickness (* _gridsize 0.1))
  (Transformation|SetRelativeScale3D (Variables|Default|Getfloor) (Utilities|NewMacro (Math|Vector|MakeVector (LocalVariables|Getwalllenght) (LocalVariables|Getwalllenght) (LocalVariables|Getwallthickness))))
  (if (Variables|wall|GetWestWall)
    (AddComponent|AddStaticMeshComponent false (Math|Transform|MakeTransform (Math|Vector|MakeVector 0.0 0.0 0.0) "0, 0, 0" (Utilities|NewMacro (Math|Vector|MakeVector (LocalVariables|Getwalllenght) (LocalVariables|Getwallthickness) (Variables|Default|Getwallheight))))))
  (if (Variables|wall|GetSouthWal)
    (AddComponent|AddStaticMeshComponent false (Math|Transform|MakeTransform (Math|Vector|MakeVector 0.0 0.0 0.0) "0, 0, 0" (Utilities|NewMacro (Math|Vector|MakeVector (LocalVariables|Getwallthickness) (LocalVariables|Getwalllenght) (Variables|Default|Getwallheight))))))
  (if (Variables|wall|GetEastWall)
    (AddComponent|AddStaticMeshComponent false (Math|Transform|MakeTransform (Math|Vector|MakeVector 0.0 (- (LocalVariables|Getwalllenght) (LocalVariables|Getwallthickness)) 0.0) "0, 0, 0" (Utilities|NewMacro (Math|Vector|MakeVector (LocalVariables|Getwalllenght) (LocalVariables|Getwallthickness) (Variables|Default|Getwallheight))))))
  (if (Variables|wall|GetNorthWall)
    (AddComponent|AddStaticMeshComponent false (Math|Transform|MakeTransform (Math|Vector|MakeVector (- (LocalVariables|Getwalllenght) (LocalVariables|Getwallthickness)) 0.0 0.0) "0, 0, 0" (Utilities|NewMacro (Math|Vector|MakeVector (LocalVariables|Getwallthickness) (LocalVariables|Getwalllenght) (Variables|Default|Getwallheight))))))
  (if (Variables|wall|Getcell)
    (AddComponent|AddStaticMeshComponent false (Math|Transform|MakeTransform (Math|Vector|MakeVector 0.0 0.0 (Variables|Default|Getwallheight)) "0, 0, 0" (Utilities|NewMacro (Math|Vector|MakeVector (Variables|Default|Getwallheight) (LocalVariables|Getwalllenght) (LocalVariables|Getwallthickness))))))
  (if (> (Variables|Default|Getlight) 0.0)
    (bind _returnvalue (AddComponent|AddPointLightComponent false (Math|Transform|MakeTransform (Math|Vector|MakeVector (* (LocalVariables|Getwalllenght) 0.5) (* (LocalVariables|Getwalllenght) 0.5) (- (Variables|Default|Getwallheight) (LocalVariables|Getwallthickness))) "0, 0, 0" "1.000000,1.000000,1.000000")))
    (bind _output_get (Variables|Default|SetPointLight _returnvalue))
    (Rendering|Components|Light|SetIntensity _output_get (Variables|Default|Getlight))
    (Rendering|Components|Light|SetLightColor _output_get (Variables|Default|GetLight%20Color) true)
    (switch Utilities|FlowControl|Switch|SwitchonTrapType (Variables|Default|GetTrap%20Type)
      (:NewEnumerator0
        (Variables|Default|SetTrap false))
      (:NewEnumerator3
        (Variables|Default|SetTrap true)
        (ChildActorComponent|SetChildActorClass (Variables|Default|GetChildActor) "/Game/Labs/Hoca_Lab/Traps/BP_TrapSpike.BP_TrapSpike_C"))
      (:NewEnumerator1
        (Variables|Default|SetTrap true)
        (ChildActorComponent|SetChildActorClass (Variables|Default|GetChildActor) "/Game/Labs/Hoca_Lab/Traps/Axe.Axe_C"))
      (:NewEnumerator2
        (Variables|Default|SetTrap true)
        (ChildActorComponent|SetChildActorClass (Variables|Default|GetChildActor) "/Game/Labs/Hoca_Lab/Traps/Gas.Gas_C")))))